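; BP_Train is a moving train hazard that kills BP_Chicken actors and destroys itself when its despawn timer runs out.
; Tick drives it forward with a swept local offset.
; CrashBox turns on physics for a living chicken's capsule and the train's HitBox, while RunOverBox squashes it flat and makes it ignore the train; both kills play a death sound.
; HornBox sounds the horn once on chicken overlap, then removes itself.
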(event OnComponentBeginOverlap(RunOverBox)
  (params (OverlappedComponent :type Primitive%20Component%20Object%20Reference) (OtherActor :type Actor%20Object%20Reference) (OtherComp :type Primitive%20Component%20Object%20Reference) (OtherBodyIndex :type Integer) (bFromSweep :type Boolean) (SweepResult :type Hit%20Result%20Structure%20%28by%20ref%29))
  (bind _self self)
  (bind _asbp_chicken (Utilities|Casting|CastToBP_Chicken OtherActor))
  (if (Variables|/Game/Blueprints/BP_Chicken.BP_Chicken_C|GetIsDead _asbp_chicken)
    (Collision|IgnoreActorwhenMoving (Variables|/Script/Engine.Character|GetCapsuleComponent _asbp_chicken) _self true)
    (else
      (Variables|/Game/Blueprints/BP_Chicken.BP_Chicken_C|SetIsDead _asbp_chicken true)
      (Collision|IgnoreActorwhenMoving (Variables|/Script/Engine.Character|GetCapsuleComponent _asbp_chicken) _self true)
      (Transformation|SetActorRelativeScale3D _asbp_chicken "1.100000,1.100000,0.001000")
      (Audio|PlaySoundatLocation "/Game/Assets/Audio/Sound_Death_V2.Sound_Death_V2" (Transformation|GetActorLocation) "0, 0, 0" 1.0 1.0 0.0 0 0 0 0))))

(event OnComponentBeginOverlap(HornBox)
  (params (OverlappedComponent :type Primitive%20Component%20Object%20Reference) (OtherActor :type Actor%20Object%20Reference) (OtherComp :type Primitive%20Component%20Object%20Reference) (OtherBodyIndex :type Integer) (bFromSweep :type Boolean) (SweepResult :type Hit%20Result%20Structure%20%28by%20ref%29))
  (Utilities|Casting|CastToBP_Chicken OtherActor)
  (Audio|PlaySoundatLocation "/Game/Assets/Audio/SCue_Train.SCue_Train" (Transformation|GetActorLocation) "0, 0, 0" 1.0 1.0 0.0 0 0 0 0)
  (Components|DestroyComponent (Variables|Default|GetHornBox)))

(event OnComponentBeginOverlap(CrashBox)
  (params (OverlappedComponent :type Primitive%20Component%20Object%20Reference) (OtherActor :type Actor%20Object%20Reference) (OtherComp :type Primitive%20Component%20Object%20Reference) (OtherBodyIndex :type Integer) (bFromSweep :type Boolean) (SweepResult :type Hit%20Result%20Structure%20%28by%20ref%29))
  (bind _asbp_chicken (Utilities|Casting|CastToBP_Chicken OtherActor))
  (if (not (Variables|/Game/Blueprints/BP_Chicken.BP_Chicken_C|GetIsDead _asbp_chicken))
    (Physics|SetSimulatePhysics (Variables|/Script/Engine.Character|GetCapsuleComponent _asbp_chicken) true)
    (Physics|SetSimulatePhysics (Variables|Default|GetHitBox) true)
    (Audio|PlaySoundatLocation "/Game/Assets/Audio/Sound_Death_V2.Sound_Death_V2" (Transformation|GetActorLocation) "0, 0, 0" 1.0 1.0 0.0 0 0 0 0)
    (Variables|/Game/Blueprints/BP_Chicken.BP_Chicken_C|SetIsDead _asbp_chicken true)))

(event EventTick
  (params (DeltaSeconds :type Float%20%28single-precision%29))
  (Transformation|AddActorLocalOffset (Math|Vector|MakeVector (* DeltaSeconds (Variables|Default|GetForwardSpeed)) 0.0 0.0) true false)
  (bind _output_get (Variables|Default|SetDespawnTimer (- (Variables|Default|GetDespawnTimer) DeltaSeconds)))
  (if (<= _output_get 0.0)
    (Actor|DestroyActor)))

(fn ConstructionScript)