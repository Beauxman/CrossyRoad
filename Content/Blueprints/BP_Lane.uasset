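; BP_Lane is one strip of an endless chicken-crossing level: grass, water, railroad or road.
; DecideLaneType picks type and meshes from the previous lane's type using weighted repeats; OnLaneSpawn randomizes direction and places coins, trees or crossing lights.
; Tick spawns logs, trains or cars on a timer, while overlap boxes remove cars and kill chickens in water.
; Chicken entry triggers the next lane, increments distance, then later sinks and destroys this lane.
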(event OnComponentBeginOverlap(TriggerZone)
  (params (OverlappedComponent :type Primitive%20Component%20Object%20Reference) (OtherActor :type Actor%20Object%20Reference) (OtherComp :type Primitive%20Component%20Object%20Reference) (OtherBodyIndex :type Integer) (bFromSweep :type Boolean) (SweepResult :type Hit%20Result%20Structure%20%28by%20ref%29))
  ;[1 1 1] Collision Handling
  (bind _asbp_chicken (Utilities|Casting|CastToBP_Chicken OtherActor))
  (Default|SpawnLaneatSpawnPoint (Variables|Default|GetLaneSpawner))
  (Components|DestroyComponent (Variables|Default|GetTriggerZone))
  (bind _result (Math|Integer|IncrementInt (Variables|/Game/Blueprints/BP_Chicken.BP_Chicken_C|GetDistance%20Count _asbp_chicken))
    (:%20%20
      (Variables|/Game/Blueprints/BP_Chicken.BP_Chicken_C|SetDistance%20Count _asbp_chicken _result)
      (Default|CallUpdateDistance _asbp_chicken)
      (Utilities|FlowControl|Delay 3e+01)
      (Components|MoveComponentTo (Variables|Default|GetStaticMesh) "0, 0,-10000.000000" "0, 0, 0" false true 5.0 false)
      (Actor|DestroyActor))))

(event OnComponentBeginOverlap(CarTrigger)
  (params (OverlappedComponent :type Primitive%20Component%20Object%20Reference) (OtherActor :type Actor%20Object%20Reference) (OtherComp :type Primitive%20Component%20Object%20Reference) (OtherBodyIndex :type Integer) (bFromSweep :type Boolean) (SweepResult :type Hit%20Result%20Structure%20%28by%20ref%29))
  ;[1 1 1] Collision Handling
  (bind _asbp_car (Utilities|Casting|CastToBP_Car OtherActor))
  (if (== OtherComp (Variables|/Game/Blueprints/BP_Car.BP_Car_C|GetHitBox _asbp_car))
    (Actor|DestroyActor _asbp_car)))

(event OnComponentBeginOverlap(CarTrigger2)
  (params (OverlappedComponent :type Primitive%20Component%20Object%20Reference) (OtherActor :type Actor%20Object%20Reference) (OtherComp :type Primitive%20Component%20Object%20Reference) (OtherBodyIndex :type Integer) (bFromSweep :type Boolean) (SweepResult :type Hit%20Result%20Structure%20%28by%20ref%29))
  ;[1 1 1] Collision Handling
  (bind _asbp_car (Utilities|Casting|CastToBP_Car OtherActor))
  (if (== (Variables|/Game/Blueprints/BP_Car.BP_Car_C|GetHitBox _asbp_car) OtherComp)
    (Actor|DestroyActor _asbp_car)))

(event OnComponentBeginOverlap(SplashBox)
  (params (OverlappedComponent :type Primitive%20Component%20Object%20Reference) (OtherActor :type Actor%20Object%20Reference) (OtherComp :type Primitive%20Component%20Object%20Reference) (OtherBodyIndex :type Integer) (bFromSweep :type Boolean) (SweepResult :type Hit%20Result%20Structure%20%28by%20ref%29))
  ;[1 1 1] Collision Handling
  (bind _asbp_chicken (Utilities|Casting|CastToBP_Chicken OtherActor))
  (if (== OtherComp (Variables|/Game/Blueprints/BP_Chicken.BP_Chicken_C|GetStaticMesh _asbp_chicken))
    (if (Math|Integer|InRange(Integer) (Variables|Default|GetLaneType) 3 4)
      (if (not (Variables|/Game/Blueprints/BP_Chicken.BP_Chicken_C|GetIsDead _asbp_chicken))
        (Collision|SetActorEnableCollision _asbp_chicken false)
        (Audio|PlaySoundatLocation "/Game/Assets/Audio/Sound_Gib.Sound_Gib" (Transformation|GetActorLocation _asbp_chicken) "0, 0, 0" 1.0 1.0 0.0 0 0 0 0)
        (Audio|PlaySoundatLocation "/Game/Assets/Audio/Sound_WaterSquawk.Sound_WaterSquawk" (Transformation|GetActorLocation _asbp_chicken) "0, 0, 0" 1.0 1.0 0.0 0 0 0 0)
        (Variables|/Game/Blueprints/BP_Chicken.BP_Chicken_C|SetIsDead _asbp_chicken true)
        (Physics|SetSimulatePhysics (Variables|/Script/Engine.Character|GetCapsuleComponent _asbp_chicken) true)))))

(event Custom|OnLaneSpawn
  (bind _returnvalue (Math|Random|RandomIntegerinRange 0 4))
  (bind _obstaclespawn1 (Variables|Default|GetObstacleSpawn1))
  (bind _obstaclespawn2 (Variables|Default|GetObstacleSpawn2))
  (bind _lanetype (Variables|Default|GetLaneType))
  (bind _obstaclespawn3 (Variables|Default|GetObstacleSpawn3))
  (bind _obstaclespawn4 (Variables|Default|GetObstacleSpawn4))
  (bind _obstaclespawn5 (Variables|Default|GetObstacleSpawn5))
  (bind _returnvalue_2 (Transformation|GetWorldLocation _obstaclespawn2))
  (bind _returnvalue_3 (Transformation|GetWorldLocation _obstaclespawn4))
  (bind _returnvalue_4 (Transformation|GetWorldLocation _obstaclespawn1))
  (bind _returnvalue_5 (Transformation|GetWorldLocation _obstaclespawn5))
  (bind _returnvalue_6 (Transformation|GetWorldLocation _obstaclespawn3))
  (bind _returnvalue_7 (Utilities|Select :Index _returnvalue :Option%200 _returnvalue_4 :Option%201 _returnvalue_2 :Option%202 _returnvalue_6 :Option%203 _returnvalue_3 :Option%204 _returnvalue_5))
  (bind _returnvalue_8 (Math|Transform|MakeTransform _returnvalue_7 "0,90.000000, 0"))
  (Variables|Default|SetLaneDirection (Math|Random|RandomBool))
  (if (== (Variables|Default|GetLaneType) 5)
    (Game|SpawnActorfromClass "/Game/Blueprints/BP_RRLight.BP_RRLight_C" (Math|Transform|MakeTransform (Transformation|GetWorldLocation (Variables|Default|GetRRCrossingSpawn)) "0, 0, 0" "1.000000,1.000000,1.000000") "Undefined" 0 0))
  ;[1 1 1] Coin Spawning
  (if (and (<= _lanetype 2) (> _lanetype 0))
    (if (<= (Math|Random|RandomIntegerinRange 0 1) 0)
      (Game|SpawnActorfromClass "/Game/Blueprints/BP_Coin.BP_Coin_C" (Math|Transform|MakeTransform (Utilities|Select :Index (Math|Random|RandomIntegerinRange 0 4) :Option%200 (Transformation|GetWorldLocation (Variables|Default|GetObstacleSpawn1)) :Option%201 (Transformation|GetWorldLocation (Variables|Default|GetObstacleSpawn2)) :Option%202 (Transformation|GetWorldLocation (Variables|Default|GetObstacleSpawn3)) :Option%203 (Transformation|GetWorldLocation (Variables|Default|GetObstacleSpawn4)) :Option%204 (Transformation|GetWorldLocation (Variables|Default|GetObstacleSpawn5))) "0,90.000000,0.000000") "AlwaysSpawn" 0 0)
      (else
        (if (<= (Variables|Default|GetLaneType) 1) :!label _label
          (if (<= (Math|Random|RandomIntegerinRange 0 2) 2)
            (Game|SpawnActorfromClass "/Game/Blueprints/BP_Tree.BP_Tree_C" (Math|Transform|MakeTransform (Math|Vector|MakeVector (.x (.location _returnvalue_8)) (.y (.location _returnvalue_8)) 9e+01) (.rotation _returnvalue_8) (.scale _returnvalue_8)) "AlwaysSpawn" 0 0)))))
    (else
      (goto _label))))

(event EventTick
  (params (DeltaSeconds :type Float%20%28single-precision%29))
  (bind _vehiclespawn2 (Variables|Default|GetVehicleSpawn2))
  (bind _lanedirection (Variables|Default|GetLaneDirection))
  (bind _vehiclespawn1 (Variables|Default|GetVehicleSpawn1))
  (bind _returnvalue (Transformation|GetWorldLocation _vehiclespawn1))
  (bind _returnvalue_2 (Transformation|GetWorldLocation _vehiclespawn2))
  (bind _returnvalue_3 (select _lanedirection _returnvalue_2 _returnvalue))
  ;[1 1 1] Vehicle Spawning
  (bind _output_get (Variables|Default|SetCarTimer (- (Variables|Default|GetCarTimer) DeltaSeconds)))
  (if (<= _output_get 0.0)
    (Variables|Default|SetCarTimer (Math|Conversions|ToFloat(Integer) (Math|Random|RandomIntegerinRange 3 5)))
    (switch int (Variables|Default|GetLaneType)
      (:3
        (bind _returnvalue_4 (Game|SpawnActorfromClass "/Game/Blueprints/BP_Log.BP_Log_C" (Math|Transform|MakeTransform _returnvalue_3 "0, 0, 0" "1.000000,1.000000,1.000000") "Undefined" 0 0 :!label _label))
        (if (Variables|Default|GetLaneDirection)
          (Transformation|AddActorLocalRotation _returnvalue_4 "0,-90.000000, 0" false false)
          (else
            (Transformation|AddActorLocalRotation _returnvalue_4 "0,90.000000, 0" false false)))
        (Variables|/Game/Blueprints/BP_Log.BP_Log_C|SetForwardSpeed _returnvalue_4 (Math|Random|RandomFloatinRange 1.5e+02 2.5e+02)))
      (:4
        (goto _label))
      (:5
        (if (== (Math|Random|RandomIntegerinRange 0 (Variables|Default|GetTrainSpawnChance)) 0)
          (bind _returnvalue_5 (Game|SpawnActorfromClass "/Game/Blueprints/BP_Train.BP_Train_C" (Math|Transform|MakeTransform _returnvalue_3 "0, 0, 0" "1.000000,1.000000,1.000000") "Undefined" 0 0))
          (if (Variables|Default|GetLaneDirection)
            (Transformation|AddActorLocalRotation _returnvalue_5 "0,-90.000000, 0" false false)
            (else
              (Transformation|AddActorLocalRotation _returnvalue_5 "0,90.000000, 0" false false)))))
      (:6
        (bind _returnvalue_6 (Game|SpawnActorfromClass "/Game/Blueprints/BP_Car.BP_Car_C" (Math|Transform|MakeTransform _returnvalue_3 "0, 0, 0" "1.000000,1.000000,1.000000") "Undefined" 0 0 :!label _label_2))
        (if (Variables|Default|GetLaneDirection)
          (Transformation|AddActorLocalRotation _returnvalue_6 "0,-90.000000, 0" false false)
          (else
            (Transformation|AddActorLocalRotation _returnvalue_6 "0,90.000000, 0" false false)))
        (Variables|/Game/Blueprints/BP_Car.BP_Car_C|SetForwardSpeed _returnvalue_6 (Math|Random|RandomFloatinRange 1.5e+02 2.5e+02)))
      (:7
        (goto _label_2))
      (:8
        (goto _label_2))
      (:9
        (goto _label_2))
      (:10
        (goto _label_2)))))

(fn ConstructionScript)

(fn DecideLaneType
  (params (PreviousLaneType :type Integer))
  (switch int PreviousLaneType
    (:0
      (CallFunction|RandomizeLaneGrass PreviousLaneType :!label _label))
    (:1
      (goto _label))
    (:2
      (goto _label))
    (:3
      (CallFunction|RandomizeLaneWater PreviousLaneType :!label _label_2))
    (:4
      (goto _label_2))
    (:5
      (CallFunction|RandomizeLaneRailroad PreviousLaneType))
    (:6
      (CallFunction|RandomizeLaneRoad PreviousLaneType :!label _label_3))
    (:7
      (goto _label_3))
    (:8
      (goto _label_3))
    (:9
      (goto _label_3))))

(fn RandomizeLaneGrass
  (params (PreviousLaneType :type Integer))
  (bind _returnvalue (Math|Random|RandomBool))
  (if (Math|Random|RandomBoolwithWeight (Variables|Default|GetRepeatChance))
    (switch int PreviousLaneType
      (:0
        (if _returnvalue
          (Variables|Default|SetLaneType 1 :!label _label)
          (else
            (Variables|Default|SetLaneType 2 :!label _label_2))))
      (:1
        (if _returnvalue
          (Variables|Default|SetLaneType 0 :!label _label_3)
          (else
            (goto _label_2))))
      (:2
        (if _returnvalue
          (goto _label_3)
          (else
            (goto _label)))))
    (CallFunction|NewLaneMesh)
    (else
      (Variables|Default|SetLaneType (Math|Random|RandomIntegerinRange 3 7))
      (CallFunction|NewLaneMesh))))

(fn RandomizeLaneWater
  (params (PreviousLaneType :type Integer))
  (if (Math|Random|RandomBoolwithWeight (Variables|Default|GetRepeatChance))
    (switch int PreviousLaneType
      (:3
        (Variables|Default|SetLaneType 4))
      (:4
        (Variables|Default|SetLaneType 3)))
    (CallFunction|NewLaneMesh)
    (else
      (bind _output_get (Variables|Default|SetLaneType (Math|Random|RandomIntegerinRange 0 5)))
      (if (>= _output_get 3)
        (Variables|Default|SetLaneType (+ (Variables|Default|GetLaneType) 2)))
      (CallFunction|NewLaneMesh))))

(fn NewLaneMesh
  (bind _lanetype (Variables|Default|GetLaneType))
  (bind _returnvalue (Utilities|Select :Index _lanetype :Option%200 "/Game/Assets/Meshes/SM_Lane_Grass.SM_Lane_Grass" :Option%201 "/Game/Assets/Meshes/SM_Lane_Grass_2.SM_Lane_Grass_2" :Option%202 "/Game/Assets/Meshes/SM_Lane_Grass_3.SM_Lane_Grass_3" :Option%203 "/Game/Assets/Meshes/SM_Lane_Water.SM_Lane_Water" :Option%204 "/Game/Assets/Meshes/SM_Lane_Water_2.SM_Lane_Water_2" :Option%205 "/Game/Assets/Meshes/SM_Lane_Railroad.SM_Lane_Railroad" :Option%206 "/Game/Assets/Meshes/SM_Lane_Road_Single.SM_Lane_Road_Single" :Option%207 "/Game/Assets/Meshes/SM_Lane_Road_Marked_Border.SM_Lane_Road_Marked_Border" :Option%208 "/Game/Assets/Meshes/SM_Lane_Road_Marked.SM_Lane_Road_Marked" :Option%209 "/Game/Assets/Meshes/SM_Lane_Road_Unmarked_Border_Flipped.SM_Lane_Road_Unmarked_Border_Flipped" :Option%2010 "/Game/Assets/Meshes/SM_Lane_Road_Unmarked_Border.SM_Lane_Road_Unmarked_Border" :Option%2011 "/Game/Assets/Meshes/SM_Lane_Road_Unmarked.SM_Lane_Road_Unmarked"))
  (Components|StaticMesh|SetStaticMesh (Variables|Default|GetStaticMesh) _returnvalue)
  (Components|StaticMesh|SetStaticMesh (Variables|Default|GetStaticMeshLeft) _returnvalue)
  (Components|StaticMesh|SetStaticMesh (Variables|Default|GetStaticMeshRight) _returnvalue))

(fn RandomizeLaneRailroad
  (params (PreviousLaneType :type Integer))
  (if (Math|Random|RandomBoolwithWeight (Variables|Default|GetRepeatChance))
    (switch int PreviousLaneType
      (:Default
        (Variables|Default|SetLaneType 5)
        (CallFunction|NewLaneMesh))
      (:5
        (bind _output_get (Variables|Default|SetLaneType (Math|Random|RandomIntegerinRange 0 6) :!label _label))
        (if (>= _output_get 5)
          (bind _result (Math|Integer|IncrementInt (Variables|Default|GetLaneType))
            (:%20%20
              (Variables|Default|SetLaneType _result))))
        (CallFunction|NewLaneMesh)))
    (else
      (goto _label))))

(fn RandomizeLaneRoad
  (params (PreviousLaneType :type Integer))
  (if (Math|Random|RandomBoolwithWeight (Variables|Default|GetRepeatChance))
    (switch int PreviousLaneType :!label _label
      (:6
        (switch int PreviousLaneType :!label _label_2
          (:6
            (Variables|Default|SetLaneType (Math|Random|RandomIntegerinRange 0 5) :!label _label_3))
          (:7
            (goto _label))
          (:8
            (Variables|Default|SetLaneType 9))
          (:9
            (goto _label_3)))
        (CallFunction|NewLaneMesh))
      (:7
        (Variables|Default|SetLaneType 8 :!label _label_4)
        (CallFunction|NewLaneMesh))
      (:8
        (goto _label_4))
      (:9
        (goto _label_2)))
    (else
      (goto _label_2))))

(fn SpawnCar
  (params (SpawnLoc :type Vector))
  (bind _returnvalue (Game|SpawnActorfromClass "/Game/Blueprints/BP_Car.BP_Car_C" (Math|Transform|MakeTransform SpawnLoc "0, 0, 0" "1.000000,1.000000,1.000000") "Undefined" 0 0))
  (Transformation|AddActorLocalRotation _returnvalue "0,90.000000, 0" false false))