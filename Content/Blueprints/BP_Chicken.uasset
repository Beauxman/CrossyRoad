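; BP_Chicken is the player-controlled chicken, which moves in discrete hops and collects coins.
; Forward and right axis input past a deadzone snaps the mesh to face that direction and moves the capsule a step with an upward offset.
; A DoOnce-guarded delay briefly blocks movement between hops.
; BeginPlay creates the HUD with a reference to the chicken, and AddCoin increments the count and fires UpdateCoin.
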(event Custom|Add%20Coin
  (Math|Integer|IncrementInt (Variables|Default|GetCoin%20Count)
    (:%20%20
      (Default|CallUpdateCoin))))

(event Custom|MovementCooldown
  ;[1 1 1] Movement Cooldown
  (Utilities|FlowControl|DoOnce false :!label _label
    (:Completed
      (Variables|Default|SetCanMove false)
      (Utilities|FlowControl|Delay 0.5)
      (Variables|Default|SetCanMove true)
      (goto _label Reset))))

(event EventBeginPlay
  ;[1 1 1] HUD
  (bind _returnvalue (UserInterface|CreateWidget "/Game/Blueprints/WBP_Hud.WBP_Hud_C"))
  (bind _output_get (Variables|Default|Sethud _returnvalue))
  (Variables|/Game/Blueprints/WBP_Hud.WBP_Hud_C|SetChicken _output_get self)
  (UserInterface|Viewport|AddtoViewport _output_get 0))

(event Input|AxisEvents|InputAxisMoveForward
  (params (AxisValue :type Float%20%28single-precision%29))
  (bind _staticmesh (Variables|Default|GetStaticMesh))
  ;[1 1 1] Movement
  (if (and (> (Math|Float|Absolute(Float) AxisValue) 0.3) (Variables|Default|GetCanMove))
    (CallFunction|MovementCooldown)
    (if (> AxisValue 0.3)
      (Transformation|SetWorldRotation _staticmesh "0,-90.000000, 0" false false)
      (else
        (Transformation|SetWorldRotation _staticmesh "0,90.000000, 0" false false)))
    (Components|MoveComponentTo (Variables|Collision|GetCapsuleComponent) (+ (Transformation|GetActorLocation) (Math|Vector|MakeVector (* AxisValue 1.5e+02) 0.0 5e+01)) "0, 0, 0" false false 0.2 false)))

(event Input|AxisEvents|InputAxisMoveRight
  (params (AxisValue :type Float%20%28single-precision%29))
  (bind _staticmesh (Variables|Default|GetStaticMesh))
  ;[1 1 1] Movement
  (if (and (> (Math|Float|Absolute(Float) AxisValue) 0.3) (Variables|Default|GetCanMove))
    (CallFunction|MovementCooldown)
    (if (> AxisValue 0.3)
      (Transformation|SetWorldRotation _staticmesh "0, 0, 0" false false)
      (else
        (Transformation|SetWorldRotation _staticmesh "0,-180.000000, 0" false false)))
    (Components|MoveComponentTo (Variables|Collision|GetCapsuleComponent) (+ (Transformation|GetActorLocation) (Math|Vector|MakeVector 0.0 (* AxisValue 1.5e+02) 5e+01)) "0, 0, 0" false false 0.2 false)))

(fn ConstructionScript)