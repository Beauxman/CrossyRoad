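; BP_Log is a moving log actor that reacts to the chicken and to other logs.
; Each tick it sweeps forward along its local X axis at ForwardSpeed and counts down a timer, destroying itself when it runs out.
; Its HitBox plays a sound when a BP_Chicken overlaps it.
; When its StaticMesh overlaps another log, both are set to the same fixed speed.
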(event OnComponentBeginOverlap(HitBox)
  (params (OverlappedComponent :type Primitive%20Component%20Object%20Reference) (OtherActor :type Actor%20Object%20Reference) (OtherComp :type Primitive%20Component%20Object%20Reference) (OtherBodyIndex :type Integer) (bFromSweep :type Boolean) (SweepResult :type Hit%20Result%20Structure%20%28by%20ref%29))
  (Utilities|Casting|CastToBP_Chicken OtherActor)
  (Audio|PlaySoundatLocation "/Game/Assets/Audio/SCue_Log.SCue_Log" (Transformation|GetActorLocation) "0, 0, 0" 1.0 1.0 0.0 0 0 0 0))

(event OnComponentBeginOverlap(StaticMesh)
  (params (OverlappedComponent :type Primitive%20Component%20Object%20Reference) (OtherActor :type Actor%20Object%20Reference) (OtherComp :type Primitive%20Component%20Object%20Reference) (OtherBodyIndex :type Integer) (bFromSweep :type Boolean) (SweepResult :type Hit%20Result%20Structure%20%28by%20ref%29))
  (bind _asbp_log (Utilities|Casting|CastToBP_Log OtherActor))
  (Variables|Default|SetForwardSpeed 2e+02)
  (Variables|BP_Log_C|SetForwardSpeed _asbp_log 2e+02))

(event EventTick
  (params (DeltaSeconds :type Float%20%28single-precision%29))
  (Transformation|AddActorLocalOffset (Math|Vector|MakeVector (* DeltaSeconds (Variables|Default|GetForwardSpeed)) 0.0 0.0) true false)
  (bind _output_get (Variables|Default|SetDespawnTimer (- (Variables|Default|GetDespawnTimer) DeltaSeconds)))
  (if (<= _output_get 0.0)
    (Actor|DestroyActor)))

(fn ConstructionScript)