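; BP_Railroad is a railroad Blueprint that alternately flashes a left and a right light, in the manner of a crossing signal.
; Tick counts down a half-second timer and toggles a boolean each time it expires.
; The boolean selects which light is set to full intensity and which drops to zero.
; The construction script is empty.
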(event EventTick
  (params (DeltaSeconds :type Float%20%28single-precision%29))
  (bind _leftlight (Variables|Default|GetLeftLight))
  (bind _rightlight (Variables|Default|GetRightLight))
  (bind _output_get (Variables|Default|SetLightTimer (- (Variables|Default|GetLightTimer) DeltaSeconds)))
  (if (<= _output_get 0.0)
    (Variables|Default|SetLightTimer 0.5)
    (bind _output_get_2 (Variables|Default|SetLight (not (Variables|Default|GetLight))))
    (if _output_get_2
      (Rendering|Components|Light|SetIntensity _leftlight 9e+03)
      (Rendering|Components|Light|SetIntensity _rightlight 0.0)
      (else
        (Rendering|Components|Light|SetIntensity _leftlight 0.0)
        (Rendering|Components|Light|SetIntensity _rightlight 9e+03)))))

(fn ConstructionScript)