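; Lane spawner that builds a chained track of BP_Lane actors and provides car spawning for it.
; On BeginPlay it spawns a starting batch, with a fixed-type first lane at the origin and each next at the newest lane's SpawnPoint.
; Each lane gets a spawner reference, and later lanes choose their type from the previous one.
; SpawnCar, not called here, places a BP_Car on a random side, rotated to match.
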(event EventBeginPlay
  (CallFunction|SpawnInitialLanes))

(event Collision|EventActorBeginOverlap
  (params (OtherActor :type Actor%20Object%20Reference)))

(event EventTick
  (params (DeltaSeconds :type Float%20%28single-precision%29)))

(fn ConstructionScript)

(fn SpawnLane
  (params (SpawnLocation :type Vector))
  (Variables|Default|SetPreviousLane (Variables|Default|GetNewestLane))
  (bind _returnvalue (Game|SpawnActorfromClass "/Game/Blueprints/BP_Lane.BP_Lane_C" (Math|Transform|MakeTransform SpawnLocation "0, 0, 0" "1.000000,1.000000,1.000000") "Undefined" 0 0))
  (bind _output_get (Variables|Default|SetNewestLane _returnvalue))
  (Variables|/Game/Blueprints/BP_Lane.BP_Lane_C|SetLaneSpawner _output_get self)
  (Default|DecideLaneType _output_get (Variables|/Game/Blueprints/BP_Lane.BP_Lane_C|GetLaneType (Variables|Default|GetPreviousLane)))
  (Default|OnLaneSpawn _output_get))

(fn SpawnLaneatSpawnPoint
  (CallFunction|SpawnLane (Transformation|GetWorldLocation (Variables|/Game/Blueprints/BP_Lane.BP_Lane_C|GetSpawnPoint (Variables|Default|GetNewestLane)))))

(fn SpawnInitialLanes
  (for _index (range 0 20)
    (Utilities|IsValid (Variables|Default|GetNewestLane)
      (:Is%20Valid
        (CallFunction|SpawnLaneatSpawnPoint))
      (:Is%20Not%20Valid
        (CallFunction|SpawnFirstLane "0, 0, 0")))))

(fn SpawnCar
  (params (SpawnLocation :type Vector))
  (bind _returnvalue (Game|SpawnActorfromClass "/Game/Blueprints/BP_Car.BP_Car_C" (Math|Transform|MakeTransform SpawnLocation "0, 0, 0" "1.000000,1.000000,1.000000") "Undefined" 0 0))
  (if (Math|Random|RandomBool)
    (Transformation|AddActorLocalOffset _returnvalue "0,400.000000,60.000000" false true)
    (Transformation|AddActorLocalRotation _returnvalue "0,-90.000000, 0" false false)
    (else
      (Transformation|AddActorLocalOffset _returnvalue "0,-400.000000,60.000000" false true)
      (Transformation|AddActorLocalRotation _returnvalue "0,90.000000, 0" false false))))

(fn SpawnFirstLane
  (params (SpawnLocation :type Vector))
  (bind _returnvalue (Game|SpawnActorfromClass "/Game/Blueprints/BP_Lane.BP_Lane_C" (Math|Transform|MakeTransform SpawnLocation "0, 0, 0" "1.000000,1.000000,1.000000") "Undefined" 0 0))
  (bind _output_get (Variables|Default|SetNewestLane _returnvalue))
  (Variables|/Game/Blueprints/BP_Lane.BP_Lane_C|SetLaneSpawner _output_get self)
  (Variables|/Game/Blueprints/BP_Lane.BP_Lane_C|SetLaneType _output_get 0)
  (Default|NewLaneMesh _output_get))